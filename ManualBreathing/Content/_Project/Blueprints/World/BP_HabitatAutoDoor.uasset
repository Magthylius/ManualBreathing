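; Automatic habitat door that opens when the player character enters its detector volume and closes when they leave.
; Overlap events on DoorDetector set a target relative position, lowering the mesh to open and returning it to the local origin to close.
; Tick continuously lerps DoorStaticMesh toward that target by a delta-time-scaled alpha, giving an eased slide without a timeline.
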(event `self.ReceiveBeginPlay`
  (set `self.TargetPosition` (`SceneComponent.RelativeLocation` (`self.DoorStaticMesh`))))

(event `self.ReceiveTick`
  (params (DeltaSeconds :type "Float (single-precision)"))
  (`SceneComponent.K2_SetRelativeLocation` (`self.DoorStaticMesh`) (`KismetMathLibrary.VLerp` (`SceneComponent.RelativeLocation` (`self.DoorStaticMesh`)) (`self.TargetPosition`) (* DeltaSeconds 7.0)) false false))

(event `self.DoorDetector.OnComponentBeginOverlap`
  (params (OverlappedComponent :type "PrimitiveComponent Object Reference") (OtherActor :type "Actor Object Reference") (OtherComp :type "PrimitiveComponent Object Reference") (OtherBodyIndex :type Integer) (bFromSweep :type Boolean) (SweepResult :type "HitResult Structure (by ref)"))
  (if (== OtherActor (`GameplayStatics.GetPlayerCharacter` 0))
    (set `self.TargetPosition` (0.0 0.0 -400.0))))

(event `self.DoorDetector.OnComponentEndOverlap`
  (params (OverlappedComponent :type "PrimitiveComponent Object Reference") (OtherActor :type "Actor Object Reference") (OtherComp :type "PrimitiveComponent Object Reference") (OtherBodyIndex :type Integer))
  (if (== OtherActor (`GameplayStatics.GetPlayerCharacter` 0))
    (set `self.TargetPosition` (0.0 0.0 0.0))))

(fn `UserConstructionScript`)